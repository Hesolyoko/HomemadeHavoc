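; BP_Agua is a configurable water hazard that builds a row of animated Paper2D flipbook tiles.
; The construction script scales the actor, clears previous components and spawns evenly spaced tiles along X, each with an optional box collider.
; At BeginPlay it binds those colliders' overlap events, which play a 2D sound and apply fixed damage to any overlapping actor, intended for the hero.
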(event `self.ReceiveBeginPlay`
  ;[1 1 1] Ao iniciar, assina o evento de colisão para cada flipbook de água criado
  ; Ao colidir com o Heroi, reproduz áudio e atribui dano total
  (add `PrimitiveComponent.OnComponentBeginOverlap` (`self.Array Colisão`) (delegate `OnComponentBeginOverlap`)))

(event `OnComponentBeginOverlap`
  (params (OverlappedComponent :type "PrimitiveComponent Object Reference") (OtherActor :type "Actor Object Reference") (OtherComp :type "PrimitiveComponent Object Reference") (OtherBodyIndex :type Integer) (bFromSweep :type Boolean) (SweepResult :type "HitResult Structure (by ref)"))
  ;[1 1 1] Ao iniciar, assina o evento de colisão para cada flipbook de água criado
  ; Ao colidir com o Heroi, reproduz áudio e atribui dano total
  (`GameplayStatics.PlaySound2D` (`self.Audio`) 1.0 1.0 0.0 null null)
  (`GameplayStatics.ApplyDamage` OtherActor 5.0))

(fn `Criar Água`
  (locals (`Local Quantidade` :type Integer))
  (bind `_tamanho_da_colisão` (`self.Tamanho da Colisão`))
  ;[1 1 1] Ajusta a quantidade correta de tiles e apaga os que foram criados anteriormente
  (set `local.Local Quantidade` (`KismetMathLibrary.Max` (- (`self.Quantidade`) 1)))
  (`self.Limpar`)
  ;[1 1 1] Cria um flipbook ao lado do outro na quantidade especificada
  (for _index (range (+ (`local.Local Quantidade`) 1))
    (bind _returnvalue (`AddComponent|NODE_AddPaperFlipbookComponent-1` :`RelativeTransform` (`KismetMathLibrary.MakeTransform` (`KismetMathLibrary.MakeVector` (* _index (`self.Distância entre tiles`))))))
    ;[1 1 1] Determina a animação do flipbook e adiciona o item na lista de flipbooks
    (`PaperFlipbookComponent.SetFlipbook` _returnvalue (`self.Flipbook`))
    (`KismetArrayLibrary.Array_Add` (`self.Array Flipbook`) _returnvalue)
    ;[1 1 1] Cria uma colisão na posição de cada tile criado
    ; Adiciona o item na lista de colisões
    ; e determina o tamanho da colisão
    (if (`self.Usa Colisão`)
      (bind _returnvalue_2 (`AddComponent|NODE_AddBoxComponent-1` :`RelativeTransform` (`KismetMathLibrary.MakeTransform` (`SceneComponent.RelativeLocation` _returnvalue))))
      (`KismetArrayLibrary.Array_Add` (`self.Array Colisão`) _returnvalue_2)
      (`BoxComponent.SetBoxExtent` _returnvalue_2 (`KismetMathLibrary.MakeVector` `_tamanho_da_colisão` `_tamanho_da_colisão` `_tamanho_da_colisão`) true))))

(fn `Limpar`
  (bind `_array_colisão` (`self.Array Colisão`))
  (bind _array_flipbook (`self.Array Flipbook`))
  (`|ExecutionSequence`
    (:`then_0`
      ;[1 1 1] Apaga os flipbooks de água criados e zera a lista de flipbooks
      (for _array_element _array_flipbook
        (`ActorComponent.K2_DestroyComponent` _array_element))
      (`KismetArrayLibrary.Array_Clear` _array_flipbook))
    (:`then_1`
      ;[1 1 1] Apaga os colisões criadas e zera a lista de colisões
      (for _array_element_2 `_array_colisão`
        (`ActorComponent.K2_DestroyComponent` _array_element_2))
      (`KismetArrayLibrary.Array_Clear` `_array_colisão`))))

(fn `UserConstructionScript`
  (bind _tamanho_geral (`self.Tamanho Geral`))
  ;[1 1 1] Determina a quantidade de tiles a serem criados e o tamanho
  ; Depois, verifica se vai usar colisão e executa a função de criar água
  (set `self.Quantidade` (`self.Quantidade`))
  (`self.SetActorScale3D` (`KismetMathLibrary.MakeVector` _tamanho_geral _tamanho_geral _tamanho_geral))
  (set `self.Usa Colisão` (`self.Usa Colisão`))
  (`self.Criar Água`))