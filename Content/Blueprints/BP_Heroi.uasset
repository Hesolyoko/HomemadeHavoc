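; BP_Heroi is the 2D side-scroller player hero, with running, jumping, melee attack, health and pause menu on input actions and mobile events.
; Tick selects flipbooks from velocity and flips control rotation.
; Delays time attack collision, hurt input lock and death, which pins the camera and calls BP_GameMode's defeat.
; Timelines shift the camera boom by direction and height, while construction applies tunable sizes, offsets and health.
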(event `self.ReceiveBeginPlay`
  ;[1 1 1] Permite o acesso ao Game Mode no início do jogo
  ; define a quantidade de pontos para a vitória e o estado de animação inicial
  (bind _asbp_game_mode (cast `/Game/Game_Mode/BP_GameMode` (`GameplayStatics.GetGameMode`)))
  (bind _output_get (set `self.As Game Mode` _asbp_game_mode))
  (set `/Game/Game_Mode/BP_GameMode.PontuacaoParaVencer` (`self.Pontuação Para Vencer`) _output_get)
  (set `self.Estados de Flipbook` "NewEnumerator0"))

(event `self.Colisão Ataque.OnComponentBeginOverlap`
  (params (OverlappedComponent :type "PrimitiveComponent Object Reference") (OtherActor :type "Actor Object Reference") (OtherComp :type "PrimitiveComponent Object Reference") (OtherBodyIndex :type Integer) (bFromSweep :type Boolean) (SweepResult :type "HitResult Structure (by ref)"))
  ;[1 1 1] Atribui Dano ao entrar em contato
  (`GameplayStatics.ApplyDamage` OtherActor 1.0))

(event `Mobile Pause`
  (bind (_audios_game_gameplay _audios_game_menuprincipal `_audios_game_vitória` _audios_game_gameover _audios_game_menupause) (break `/Game/Audio/AudiosDoJogo` (`self.Audios Game`)))
  ;[1 1 1] Ativa o Menu de Pause na tela
  (`GameplayStatics.PlaySound2D` _audios_game_menupause 1.0 1.0 0.0 null null :!label _label)
  (bind _returnvalue (`|CreateWidget` "/Game/UI/MenuPause.MenuPause_C" (`GameplayStatics.GetPlayerController` 0)))
  (`UserWidget.AddToViewport` _returnvalue 2))

(event `Mobile Ataque`
  (bind _audios_do_heroi_ataque (break `/Game/Audio/AudiosDoHeroi` (`self.Audios do Heroi`)))
  ;[1 1 1] Muda para o flipbook de ataque, reproduz o áudio e marca como verdadeiro a variável de ataque para interromper o movimento do Heroi
  ; Depois, liga a colisão da colisão do ataque e aguarda o delay de animação de ataque
  ; Ao fim, desliga colisão e desliga a variável para voltar ao movimento
  (set `self.bEstaAtacando` true :!label _label_2)
  (`/Engine/EditorBlueprintResources/StandardMacros.DoOnce` false :!label _label_3
    (:`Completed`
      (`PaperFlipbookComponent.SetFlipbook` (`self.Sprite`) (`self.Atacando`))
      (`GameplayStatics.PlaySound2D` _audios_do_heroi_ataque 1.0 1.0 0.0 null null)
      (`PrimitiveComponent.SetCollisionEnabled` (`self.Colisão Ataque`) "QueryOnly")
      (`KismetSystemLibrary.Delay` (`self.Duração da animação de ataque`))
      (`PrimitiveComponent.SetCollisionEnabled` (`self.Colisão Ataque`) "NoCollision")
      (set `self.bEstaAtacando` false)
      (goto _label_3 :!via `Reset`))))

(event `InputAction|Pause`
  (params (Key :type "Key Structure"))
  ;[1 1 1] Ativa o Menu de Pause na tela
  (:`Pressed`
    (goto _label)))

(event `InputAction|Attack`
  (params (Key :type "Key Structure"))
  ;[1 1 1] Muda para o flipbook de ataque, reproduz o áudio e marca como verdadeiro a variável de ataque para interromper o movimento do Heroi
  ; Depois, liga a colisão da colisão do ataque e aguarda o delay de animação de ataque
  ; Ao fim, desliga colisão e desliga a variável para voltar ao movimento
  (:`Pressed`
    (goto _label_2)))

(event `self.ReceiveAnyDamage`
  (params (Damage :type "Float (single-precision)") (DamageType :type "DamageType Object Reference") (InstigatedBy :type "Controller Object Reference") (DamageCauser :type "Actor Object Reference"))
  (bind _returnvalue (`KismetMathLibrary.GetForwardVector` (`self.K2_GetActorRotation`)))
  ;[1 1 1] Recebe Dano e atualiza a vida no HUD, depois verifica o estado atual da vida
  ; Se zerou, ativa a variável de morte e chama o evento Morreu
  ; Se não zerou, arremessa o Heroi, ativa a variável de Dano e chama o evento de animação de dano
  (bind _output_get (set `self.Vida Atual` (`KismetMathLibrary.FClamp` (- (`self.Vida Atual`) Damage) 0.0 (`self.Vida Máxima`))))
  (`self.Atualiza Vida`)
  (bind _returnvalue_2 (<= _output_get 0.0))
  (if _returnvalue_2
    (set `self.bEstaMorto` true)
    (`self.Morreu`)
    (else
      (bind (_returnvalue_x _returnvalue_y) (`KismetMathLibrary.BreakVector` (select `bool` _returnvalue_2 :`false` (* _returnvalue -1500) :`true` (* _returnvalue 0))))
      (`self.LaunchCharacter` (`KismetMathLibrary.MakeVector` _returnvalue_x _returnvalue_y 600.0) true true)
      (set `self.bEstaEmAnimacaoDeDano` true)
      (`self.Recebeu Dano`))))

(event `Morreu`
  (bind (_audios_do_heroi_ataque _audios_do_heroi_pulo _audios_do_heroi_sofrendodano _audios_do_heroi_morte) (break `/Game/Audio/AudiosDoHeroi` (`self.Audios do Heroi`)))
  ;[1 1 1] Executa o evento de Morte que determina a posição da câmera na posição em que o Heroi morreu
  ; Reproduz o áudio e para o movimento, depois troca o flipbook de animação de morte
  ; Desabilita os inputs e a colisão do Heroi
  ; Aguarda o delay de animação de morte e troca para o flipbook de morto
  ; Ao fim, chama o evento de Derrota na HUD Gameplay
  (`PaperFlipbookComponent.SetFlipbook` (`self.Sprite`) (`self.Morrendo`))
  (set `self.PosicaoDaCameraAoMorrer` (`SceneComponent.K2_GetComponentLocation` (`self.CameraBoom`)))
  (`GameplayStatics.PlaySound2D` _audios_do_heroi_morte 1.0 1.0 0.0 null null)
  (`MovementComponent.StopMovementImmediately` (`self.CharacterMovement`))
  (`self.DisableInput` (`GameplayStatics.GetPlayerController` 0))
  (`PrimitiveComponent.SetCollisionEnabled` (`self.CapsuleComponent`) "NoCollision")
  (`KismetSystemLibrary.Delay` (`self.Duração da animação de morte`))
  (`PaperFlipbookComponent.SetFlipbook` (`self.Sprite`) (`self.Morto`))
  (`/Game/Game_Mode/BP_GameMode.Derrota` (`self.As Game Mode`)))

(event `InputAxis|MoveRight`
  (params (AxisValue :type "Float (single-precision)"))
  ;[1 1 1] Verifica se o personagem está andando para esquerda ou direita, informa que ele está se movendo, adiciona movimento e executa o evento para ajustar camera.
  (if (> AxisValue 0.0)
    (set `self.bAndaParaDireita` true)
    (elif (< AxisValue 0.0)
      (set `self.bAndaParaDireita` false)))
  (set `self.bEstaSeMovendo` (!= AxisValue 0.0))
  (`self.AddMovementInput` (1.0 0.0 0.0) AxisValue)
  (`self.Ajusta Camera`))

(event `Recebeu Dano`
  (bind (_audios_do_heroi_ataque _audios_do_heroi_pulo _audios_do_heroi_sofrendodano) (break `/Game/Audio/AudiosDoHeroi` (`self.Audios do Heroi`)))
  ;[1 1 1] Executa o evento de animação de dano, reproduz o áudio e desabilita os inputs
  ; Troca o flipbook para a animação de dano
  ; Aguarda o delay da animação de dano e habilita novamente os inputs
  ; Ao fim, desliga a variável de dano para retornar ao movimento
  (`GameplayStatics.PlaySound2D` _audios_do_heroi_sofrendodano 1.0 1.0 0.0 null null)
  (`self.DisableInput` (`GameplayStatics.GetPlayerController` 0))
  (`PaperFlipbookComponent.SetFlipbook` (`self.Sprite`) (`self.Sofrendo Dano`))
  (`KismetSystemLibrary.Delay` (`self.Duração da animação de dano`))
  (`self.EnableInput` (`GameplayStatics.GetPlayerController` 0))
  (set `self.bEstaEmAnimacaoDeDano` false))

(event `Mobile Jump`
  (bind (_audios_do_heroi_ataque _audios_do_heroi_pulo) (break `/Game/Audio/AudiosDoHeroi` (`self.Audios do Heroi`)))
  ;[1 1 1] Aciona o pulo do personagem e reproduz o áudio
  ; Ao tocar o chão, reseta o Do Once para poder reproduzir o áudio no próximo pulo
  (`/Engine/EditorBlueprintResources/StandardMacros.DoOnce` false :!label _label_4
    (:`Completed`
      (`GameplayStatics.PlaySound2D` _audios_do_heroi_pulo 1.0 1.0 0.0 null null)
      (`self.Jump`))))

(event `Ajusta Camera`
  (bind (_returnvalue_x _returnvalue_y _returnvalue_z) (`KismetMathLibrary.BreakVector` (`self.K2_GetActorLocation`)))
  (bind `_posição_vertical_da_camera` (`self.Posição vertical da camera`))
  (bind `_posição_horizontal_da_camera` (`self.Posição horizontal da camera`))
  ;[1 1 1] Verifica se o Heroi está se movendo e define a animação de posicionamento da camera para manter o jogador sempre no canto da tela e ajustar a distância da camera
  (`|ExecutionSequence`
    (:`then_0`
      (if (`self.bEstaSeMovendo`)
        (`TimelineComponent.SetPlayRate` (`self.Camera Boom Horizontal`) (/ 1.0 (`self.Tempo de animação da camera`)))
        (if (`self.bAndaParaDireita`)
          (bind (_direction _alpha) (`Timeline|Camera Boom Horizontal` :!via `Reverse` :!label _label_5)
            (:`Update`
              (set `SpringArmComponent.SocketOffset` (`KismetMathLibrary.VLerp` (`KismetMathLibrary.MakeVector` 0.0 `_posição_horizontal_da_camera` `_posição_vertical_da_camera`) (`KismetMathLibrary.MakeVector` 0.0 (* `_posição_horizontal_da_camera` -1.0) `_posição_vertical_da_camera`) _alpha) (`self.CameraBoom`))))
          (else
            (goto _label_5)))))
    (:`then_1`
      (`TimelineComponent.SetPlayRate` (`self.Camera Boom Profundidade`) (/ 1.0 (`self.Tempo de animação da camera`)))
      (`/Engine/EditorBlueprintResources/StandardMacros.CompareFloat` (`KismetMathLibrary.MapRangeUnclamped` _returnvalue_z 400.0 1000.0 0.0 1.0) 0.5
        (:`>`
          (bind (_direction_2 _alpha_2) (`Timeline|Camera Boom Profundidade` :!label _label_6)
            (:`Update`
              (set `SpringArmComponent.TargetArmLength` (`KismetMathLibrary.Lerp` (`self.Distância da Camera de Perto`) (`self.Distância da Camera de Longe`) _alpha_2) (`self.CameraBoom`)))))
        (:`<`
          (goto _label_6 :!via `Reverse`))))))

(event `InputAction|Jump`
  (params (Key :type "Key Structure"))
  ;[1 1 1] Aciona o pulo do personagem e reproduz o áudio
  ; Ao tocar o chão, reseta o Do Once para poder reproduzir o áudio no próximo pulo
  (:`Pressed`
    (goto _label_4))
  (:`Released`
    (`self.StopJumping`)))

(event `self.ReceiveTick`
  (params (DeltaSeconds :type "Float (single-precision)"))
  ;[1 1 1] Verifica se o Heroi está morto
  ; Se verdadeiro, pega a posição em que a camera estava ao morrer e fixa ela na posição
  ; Se falso, executa função de atualizar flipbooks e atualiza rotação do personagem conforme o lado para o qual está andando.
  (if (`self.bEstaMorto`)
    (`SceneComponent.K2_SetWorldLocation` (`self.CameraBoom`) (`self.PosicaoDaCameraAoMorrer`) false false)
    (else
      (`|ExecutionSequence`
        (:`then_0`
          (`self.Atualiza Flipbooks`))
        (:`then_1`
          (`self.Atualiza Rotação`))))))

(event `self.OnLanded`
  (params (Hit :type "HitResult Structure (by ref)"))
  ;[1 1 1] Aciona o pulo do personagem e reproduz o áudio
  ; Ao tocar o chão, reseta o Do Once para poder reproduzir o áudio no próximo pulo
  (`self.StopJumping`)
  (goto _label_4 :!via `Reset`))

(fn `Atualiza Flipbooks`
  (bind (_returnvalue_x _returnvalue_y _returnvalue_z) (`KismetMathLibrary.BreakVector` (`self.GetVelocity`)))
  (bind (_returnvalue_x_2 _returnvalue_y_2 _returnvalue_z_2) (`KismetMathLibrary.BreakVector` (`self.GetVelocity`)))
  ;[1 1 1] Verifica se está em animação de dano ou de ataque e interrompe o movimento
  (if (or (`self.bEstaEmAnimacaoDeDano`) (`self.bEstaAtacando`))
    (if (not (!= _returnvalue_z_2 0.0))
      (`MovementComponent.StopMovementImmediately` (`self.CharacterMovement`)))
    (else
      ;[1 1 1] Atribui na variável o nome do estado verificado
      (set `self.Estados de Flipbook` (select `bool` (!= (`KismetMathLibrary.VSize` (`self.GetVelocity`)) 0.0) :`false` "NewEnumerator1" :`true` (select `bool` (`NavMovementComponent.IsFalling` (`self.CharacterMovement`)) :`false` "NewEnumerator2" :`true` (select `bool` (<= _returnvalue_z 0.0) :`false` "NewEnumerator4" :`true` "NewEnumerator3" :!type "/Game/Game_Mode/EMovimentos Enum"))))
      ;[1 1 1] Muda o flipbook de animação conforme a mudança do nome de estado na variável
      (`PaperFlipbookComponent.SetFlipbook` (`self.Sprite`) (select `/Game/Game_Mode/EMovimentos` (`self.Estados de Flipbook`) :`NewEnumerator1` (`self.Idle`) :`NewEnumerator2` (`self.Correndo`) :`NewEnumerator3` (`self.Caindo`) :`NewEnumerator4` (`self.Pulando`))))))

(fn `Atualiza Rotação`
  (bind _returnvalue_x (`KismetMathLibrary.BreakVector` (`self.GetVelocity`)))
  (bind _returnvalue (`GameplayStatics.GetPlayerController` 0))
  ;[1 1 1] Verifica o movimento do personagem e muda a rotação do Heroi
  (`/Engine/EditorBlueprintResources/StandardMacros.CompareFloat` _returnvalue_x
    (:`>`
      (`Controller.SetControlRotation` _returnvalue (`KismetMathLibrary.MakeRotator` 0.0)))
    (:`<`
      (`Controller.SetControlRotation` _returnvalue (`KismetMathLibrary.MakeRotator` 0.0 0.0 180.0)))))

(fn `Atualiza Vida`
  ;[1 1 1] Chama a função de atualizar vida dentro do HUD Vida
  ; OBS: O HUD Vida é executado dentro do HUD Gameplay, que no caso está sendo executado de dentro do Game Mode
  (`/Game/UI/HUD_Vida.Atualiza Vida` (`/Game/UI/HUD_Gameplay.HUD_Vida` (`/Game/Game_Mode/BP_GameMode.HUD Gameplay` (`self.As Game Mode`))) (`self.Vida Atual`)))

(fn `UserConstructionScript`
  (bind _tamanho_do_sprite (`self.Tamanho do Sprite`))
  (bind `_colisão_ataque` (`self.Colisão Ataque`))
  (bind _tamanho_geral (`self.Tamanho Geral`))
  (bind _capsulecomponent (`self.CapsuleComponent`))
  ;[1 1 1] Inicia a configuração na instância do jogo
  (`PaperFlipbookComponent.SetFlipbook` (`self.Sprite`) (`self.Idle`))
  (`self.SetActorScale3D` (`KismetMathLibrary.MakeVector` _tamanho_geral _tamanho_geral _tamanho_geral))
  (set `self.Vida Atual` (`self.Vida Máxima`))
  (`SphereComponent.SetSphereRadius` `_colisão_ataque` (`self.Tamanho da colisão do ataque`) true)
  (`SceneComponent.K2_SetRelativeLocation` `_colisão_ataque` (`KismetMathLibrary.MakeVector` (`self.Posição do ataque Horizontal`) 0.0 (`self.Posição do ataque Vertical`)) false false)
  (`CapsuleComponent.SetCapsuleHalfHeight` _capsulecomponent (`self.Altura da colisão do Heroi`) true)
  (`CapsuleComponent.SetCapsuleRadius` _capsulecomponent (`self.Largura da colisão do Heroi`) true)
  (`SceneComponent.SetRelativeScale3D` (`self.Sprite`) (`KismetMathLibrary.MakeVector` _tamanho_do_sprite _tamanho_do_sprite _tamanho_do_sprite))
  (set `SpringArmComponent.SocketOffset` (`KismetMathLibrary.MakeVector` 0.0 (`self.Posição horizontal da camera`) (`self.Posição vertical da camera`)) (`self.CameraBoom`))
  (`SceneComponent.K2_SetRelativeLocation` (`self.Sprite`) (`KismetMathLibrary.MakeVector` (`self.Posição Horizontal do Sprite`) 0.0 (`self.Posição Vertical do Sprite`)) false false))