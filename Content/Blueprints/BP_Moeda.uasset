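; BP_Moeda is a collectible coin with an animated Paper2D flipbook that awards a point when the hero touches it.
; The construction script applies the configurable flipbook, overall scale, sprite offset and capsule size.
; BeginPlay caches BP_GameMode and randomizes the flipbook's start time.
; Capsule overlap with BP_Heroi plays a sound, then, if the game mode is valid, calls GanharPonto and destroys the coin.
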(event `self.ReceiveBeginPlay`
  ;[1 1 1] Chama o Game Mode e determina um valor aleatória para o tempo de animação do flipbook
  (bind _asbp_game_mode (cast `/Game/Game_Mode/BP_GameMode` (`GameplayStatics.GetGameMode`)))
  (set `self.As Toolkit Game Mode` _asbp_game_mode)
  (`PaperFlipbookComponent.SetNewTime` (`self.PaperFlipbook`) (`KismetMathLibrary.RandomFloat`)))

(event `self.Capsule.OnComponentBeginOverlap`
  (params (OverlappedComponent :type "PrimitiveComponent Object Reference") (OtherActor :type "Actor Object Reference") (OtherComp :type "PrimitiveComponent Object Reference") (OtherBodyIndex :type Integer) (bFromSweep :type Boolean) (SweepResult :type "HitResult Structure (by ref)"))
  ;[1 1 1] Ao colidir com o Heroi, reproduz o áudio
  ; depois, verifica o game mode e chama a função de atribuir ponto e checar vitória
  ; ao final, destrói a moeda
  (cast `/Game/Blueprints/BP_Heroi` OtherActor)
  (`GameplayStatics.PlaySound2D` (`self.Audio`) 1.0 1.0 0.0 null null)
  (bind _as_toolkit_game_mode (`self.As Toolkit Game Mode`)
    (:`then`
      (`/Game/Game_Mode/BP_GameMode.Ganhar Ponto` _as_toolkit_game_mode 1)
      (`self.K2_DestroyActor`))
    (:`else`)))

(fn `UserConstructionScript`
  (bind _tamanho_geral (`self.Tamanho Geral`))
  (bind _capsule (`self.Capsule`))
  ;[1 1 1] Determina o flipbook e o tamanho geral da moeda
  ; depois, define a posição do sprite
  ; por fim, ajusta o tamanho da colisão
  (`PaperFlipbookComponent.SetFlipbook` (`self.PaperFlipbook`) (`self.Flipbook`))
  (`self.SetActorScale3D` (`KismetMathLibrary.MakeVector` _tamanho_geral _tamanho_geral _tamanho_geral))
  (`SceneComponent.K2_SetRelativeLocation` (`self.PaperFlipbook`) (`KismetMathLibrary.MakeVector` (`self.Posição Horizontal do Sprite`) 0.0 (`self.Posição Vertical do Sprite`)) false false)
  (`CapsuleComponent.SetCapsuleHalfHeight` _capsule (`self.Altura da colisão`) true)
  (`CapsuleComponent.SetCapsuleRadius` _capsule (`self.Largura da colisão`) true))