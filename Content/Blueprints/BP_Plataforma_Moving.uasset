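; Paper2D platform that moves between its start position and a horizontal/vertical offset, and can optionally vanish when the hero stands on it.
; A timeline drives movement at a rate set by the travel time.
; With the timer enabled, sensor overlap starts, after a short delay, a color warning and countdown to hide, play audio and later reappear; leaving cancels the countdown.
; The construction script applies sprite, flip, scale and sensor bounds.
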(event `self.ReceiveBeginPlay`
  (bind (`_posição_inicial_x` `_posição_inicial_y` `_posição_inicial_z`) (`KismetMathLibrary.BreakVector` (`self.Posição Inicial`)))
  ;[1 1 1] Configura a caixa de colisão da plataforma
  ; se for uma plataforma que some com o tempo liga a colisão
  ; se não, desliga a colisão para economizar processamento
  (`PrimitiveComponent.SetCollisionEnabled` (`self.Sensor`) (select `bool` (`self.bUsaTemporizador`) :`false` "NoCollision" :`true` "QueryOnly" :!type "ECollisionEnabled Enum"))
  ;[1 1 1] Define a posição inicial da plataforma e o tempo da animação
  ; Inicializa a animação de movimento Horizontal e Vertical
  (set `self.Posição Inicial` (`self.K2_GetActorLocation`))
  (`TimelineComponent.SetPlayRate` (`self.Timeline Movimento`) (/ 1.0 (`self.Tempo do Movimento`)))
  (bind (_direction _alpha) (`Timeline|Timeline Movimento`)
    (:`Update`
      (`self.K2_SetActorLocation` (`KismetMathLibrary.VLerp` (`self.Posição Inicial`) (`KismetMathLibrary.MakeVector` (+ `_posição_inicial_x` (`self.Destino Horizontal`)) `_posição_inicial_y` (+ `_posição_inicial_z` (`self.Destino Vertical`))) _alpha)))))

(event `self.Sensor.OnComponentBeginOverlap`
  (params (OverlappedComponent :type "PrimitiveComponent Object Reference") (OtherActor :type "Actor Object Reference") (OtherComp :type "PrimitiveComponent Object Reference") (OtherBodyIndex :type Integer) (bFromSweep :type Boolean) (SweepResult :type "HitResult Structure (by ref)"))
  ;[1 1 1] Verifica a colisção com o Heroi
  ; Após um delay de 0.6 segundos, inicializa a animação que serve de feedback para o jogador saber que a plataforma será destruída
  ; Inicializa a contagem para a destruição
  ; Ao destruir, desliga a visibilidade e a colisão
  ; Depois, reproduz áudio e inicia contagem para reaparecer
  (cast `/Game/Blueprints/BP_Heroi` OtherActor)
  (`KismetSystemLibrary.Delay` 0.6)
  (`KismetSystemLibrary.K2_ClearAndInvalidateTimerHandle` (`self.Temporizador`))
  (`|ExecutionSequence`
    (:`then_0`
      (bind (_direction _cor) (`Timeline|Timeline Cor` :!via `PlayFromStart`)
        (:`Update`
          (`PaperSpriteComponent.SetSpriteColor` (`self.PaperSprite`) _cor))))
    (:`then_1`
      (bind _returnvalue (`KismetSystemLibrary.K2_SetTimerDelegate` (delegate `DestruirPlataforma`) (`self.TempoParaDestruir`)))
      (set `self.Temporizador` _returnvalue))))

(event `DestruirPlataforma`
  ;[1 1 1] Verifica a colisção com o Heroi
  ; Após um delay de 0.6 segundos, inicializa a animação que serve de feedback para o jogador saber que a plataforma será destruída
  ; Inicializa a contagem para a destruição
  ; Ao destruir, desliga a visibilidade e a colisão
  ; Depois, reproduz áudio e inicia contagem para reaparecer
  (`self.SetActorHiddenInGame` true)
  (`self.SetActorEnableCollision` false)
  (`GameplayStatics.PlaySound2D` (`self.Audio`) 1.0 1.0 0.0 null null)
  (`KismetSystemLibrary.K2_SetTimerDelegate` (delegate `Reaparecer`) (`self.TempoParaReaparecer`)))

(event `Reaparecer`
  ;[1 1 1] Verifica a colisção com o Heroi
  ; Após um delay de 0.6 segundos, inicializa a animação que serve de feedback para o jogador saber que a plataforma será destruída
  ; Inicializa a contagem para a destruição
  ; Ao destruir, desliga a visibilidade e a colisão
  ; Depois, reproduz áudio e inicia contagem para reaparecer
  (`self.SetActorHiddenInGame` false)
  (`self.SetActorEnableCollision` true)
  (`self.CancelarTemporizador`))

(event `self.Sensor.OnComponentEndOverlap`
  (params (OverlappedComponent :type "PrimitiveComponent Object Reference") (OtherActor :type "Actor Object Reference") (OtherComp :type "PrimitiveComponent Object Reference") (OtherBodyIndex :type Integer))
  ;[1 1 1] Se o jogador parar de colidir com a plataforma, para a contagem de destruição.
  (cast `/Game/Blueprints/BP_Heroi` OtherActor)
  (`self.CancelarTemporizador`))

(event `CancelarTemporizador`
  ;[1 1 1] Cancela e invalida o temporizador, para a animação de feedback de destruição e força o sprite a voltar para a cor original.
  (`KismetSystemLibrary.K2_ClearAndInvalidateTimerHandle` (`self.Temporizador`))
  (`TimelineComponent.Stop` (`self.Timeline Cor`))
  (`PaperSpriteComponent.SetSpriteColor` (`self.PaperSprite`) (struct :`R` 1.0 :`G` 1.0 :`B` 1.0 :`A` 1.0)))

(fn `UserConstructionScript`
  (bind _tamanho (`self.Tamanho`))
  ;[1 1 1] Determina o Sprite a ser usado, verifica a variável para inverter o Sprite e configura o tamanho geral
  ; Depois define o tamanho do sensor e a posição
  (`PaperSpriteComponent.SetSprite` (`self.PaperSprite`) (`self.Sprite`))
  (`self.SetActorScale3D` (`KismetMathLibrary.MakeVector` (* (`KismetMathLibrary.SelectFloat` -1.0 1.0 (`self.bInverterSprite`)) _tamanho) _tamanho _tamanho))
  (`BoxComponent.SetBoxExtent` (`self.Sensor`) (`KismetMathLibrary.MakeVector` (`self.Tamanho Horizontal do Sensor`) 0.0 (`self.Tamanho Vertical do Sensor`)) true)
  (`SceneComponent.K2_SetRelativeLocation` (`self.Sensor`) (`KismetMathLibrary.MakeVector` (`self.Posição Horizontal do Sensor`) 0.0 (`self.Posição Vertical do Sensor`)) false false))