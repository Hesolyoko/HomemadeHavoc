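; BP_Vida is a 2D health pickup that restores one life to BP_Heroi, up to a maximum of three.
; Capsule overlap below that maximum increments VidaAtual, calls AtualizaVida for the HUD, plays a sound and hides the pickup without collision.
; A timer restores visibility and collision after TempoParaReaparecer, reusing the actor instead of respawning it.
; The construction script applies configurable flipbook, scale, sprite offset and capsule size.
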(event `self.Capsule.OnComponentBeginOverlap`
  (params (OverlappedComponent :type "PrimitiveComponent Object Reference") (OtherActor :type "Actor Object Reference") (OtherComp :type "PrimitiveComponent Object Reference") (OtherBodyIndex :type Integer) (bFromSweep :type Boolean) (SweepResult :type "HitResult Structure (by ref)"))
  ;[1 1 1] Ao colidir com o Heroi, verifica se a vida está no máximo
  ; Se não estiver, acrescenta uma vida (até atingir o máximo de 3)
  ; Depois, atualiza a variável de vida do Heroi e chama a função para atualizar vida no HUD
  (bind _asbp_heroi (cast `/Game/Blueprints/BP_Heroi` OtherActor))
  (bind _vida_atual (`/Game/Blueprints/BP_Heroi.Vida Atual` _asbp_heroi))
  (`/Engine/EditorBlueprintResources/StandardMacros.CompareFloat` _vida_atual 3.0
    (:`<`
      (bind _result (`/Engine/EditorBlueprintResources/StandardMacros.IncrementFloat` _vida_atual)
        (:`  `
          (set `/Game/Blueprints/BP_Heroi.Vida Atual` (`KismetMathLibrary.FClamp` _result 0.0 3.0) _asbp_heroi)
          (`/Game/Blueprints/BP_Heroi.Atualiza Vida` _asbp_heroi)
          ;[1 1 1] Reproduz o áudio, desliga a colisão e a visualização
          (`GameplayStatics.PlaySound2D` (`self.Audio`) 1.0 1.0 0.0 null null)
          (`self.SetActorEnableCollision` false)
          (`self.SetActorHiddenInGame` true)
          ;[1 1 1] Se estiver usando temporizador, conta o tempo determinado para reaparecer e devolve a colisão e a visibilidade
          (`KismetSystemLibrary.K2_SetTimerDelegate` (delegate `Reaparecer`) (`self.TempoParaReaparecer`)))))))

(event `Reaparecer`
  ;[1 1 1] Se estiver usando temporizador, conta o tempo determinado para reaparecer e devolve a colisão e a visibilidade
  (`self.SetActorHiddenInGame` false)
  (`self.SetActorEnableCollision` true))

(fn `UserConstructionScript`
  (bind _tamanho_geral (`self.Tamanho Geral`))
  (bind _capsule (`self.Capsule`))
  ;[1 1 1] Configura o flipbook a ser usado e o tamanho geral
  ; depois, define a posição do sprite
  ; por fim, ajusta o tamanho da colisão
  (`PaperFlipbookComponent.SetFlipbook` (`self.Vida`) (`self.Flipbook`))
  (`self.SetActorScale3D` (`KismetMathLibrary.MakeVector` _tamanho_geral _tamanho_geral _tamanho_geral))
  (`SceneComponent.K2_SetRelativeLocation` (`self.Vida`) (`KismetMathLibrary.MakeVector` (`self.Posição Horizontal do Sprite`) 0.0 (`self.Posição Vertical do Sprite`)) false false)
  (`CapsuleComponent.SetCapsuleHalfHeight` _capsule (`self.Altura da colisão`) true)
  (`CapsuleComponent.SetCapsuleRadius` _capsule (`self.Largura da colisão`) true))