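; Paper2D patrolling enemy that walks along X from a random starting direction and damages player 0 on contact.
; Capsule hits with other actors on an X-facing normal reverse movement and mirror the sprite; delayed DoOnce resets debounce turns and throttle contact damage.
; Taking damage flashes the sprite color via a timeline, while zero health disables collision, plays death flipbook and sound, then destroys it.
; The construction script applies health, flipbook, scale, capsule and sprite settings from variables.
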(event `self.ReceiveBeginPlay`
  ;[1 1 1] Ao iniciar o jogo, escolhe uma direção aleatória para o movimento
  (set `self.bInverterDireção` (`KismetMathLibrary.RandomBool`))
  (`self.Muda Direção`))

(event `self.ReceiveAnyDamage`
  (params (Damage :type "Float (single-precision)") (DamageType :type "DamageType Object Reference") (InstigatedBy :type "Controller Object Reference") (DamageCauser :type "Actor Object Reference"))
  ;[1 1 1] Recebe Dano e verifica a quantidade de vida
  ; Se zerou, executa morte
  ; Se não, muda cor do inimigo para identificar que recebeu dano
  (bind _output_get (set `self.Vida Atual` (`KismetMathLibrary.FClamp` (- (`self.Vida Atual`) Damage) 0.0 (`self.Vida Máxima`))))
  (if (<= _output_get 0.0)
    (`self.Inimigo Morreu`)
    (`KismetSystemLibrary.Delay` 0.7)
    (`self.K2_DestroyActor`)
    (else
      (bind (_direction _cor) (`Timeline|Timeline_0`)
        (:`Update`
          (`PaperFlipbookComponent.SetSpriteColor` (`self.Sprite`) _cor))
        (:`Finished`
          (`PaperFlipbookComponent.SetSpriteColor` (`self.Sprite`) (struct :`R` 1.0 :`G` 1.0 :`B` 1.0 :`A` 1.0)))))))

(event `self.ReceiveTick`
  (params (DeltaSeconds :type "Float (single-precision)"))
  ;[1 1 1] Verifica a variável de inverter direção e adiciona movimento
  (`self.AddMovementInput` (1.0 0.0 0.0) (select `bool` (`self.bInverterDireção`) :`false` -1.0 :`true` 1.0 :!type "Float (single-precision)")))

(event `self.CapsuleComponent.OnComponentHit`
  (params (HitComponent :type "PrimitiveComponent Object Reference") (OtherActor :type "Actor Object Reference") (OtherComp :type "PrimitiveComponent Object Reference") (NormalImpulse :type "Vector Structure") (Hit :type "HitResult Structure (by ref)"))
  (bind _returnvalue (`GameplayStatics.GetPlayerPawn` 0))
  ;[1 1 1] Verifica se o contato foi com o Heroi ou não
  (if (!= OtherActor _returnvalue)
    ;[1 1 1] Se o contato não for com o Heroi, muda de direção e continua se movimentando
    (if (!= (.x Hit_Normal) 0.0)
      (`/Engine/EditorBlueprintResources/StandardMacros.DoOnce` false :!label _label
        (:`Completed`
          (set `self.bInverterDireção` (not (`self.bInverterDireção`)))
          (`self.Muda Direção`)
          (`KismetSystemLibrary.Delay` 0.1)
          (`self.Reseta Mudança de Direção`))))
    (else
      ;[1 1 1] Aplica Dano se o contato for com o Heroi e aguarda meio segundo até aplicar o dano novamente
      (`/Engine/EditorBlueprintResources/StandardMacros.DoOnce` false :!label _label_2
        (:`Completed`
          (`GameplayStatics.ApplyDamage` _returnvalue 1.0)
          (`KismetSystemLibrary.Delay` 0.5)
          (goto _label_2 :!via `Reset`))))))

(event `Reseta Mudança de Direção`
  ;[1 1 1] Se o contato não for com o Heroi, muda de direção e continua se movimentando
  (goto _label :!via `Reset`))

(fn `Inimigo Morreu`
  ;[1 1 1] Desliga a colisão do inimigo, muda para a animação de morte e reproduz o áudio
  (`PrimitiveComponent.SetCollisionEnabled` (`self.CapsuleComponent`) "NoCollision")
  (`PaperFlipbookComponent.SetFlipbook` (`self.Sprite`) (`self.Morte`))
  (`GameplayStatics.PlaySound2D` (`self.Audio`) 1.0 1.0 0.0 null null))

(fn `Muda Direção`
  (bind (_returnvalue_x _returnvalue_y _returnvalue_z) (`KismetMathLibrary.BreakVector` (`SceneComponent.K2_GetComponentScale` (`self.Sprite`))))
  ;[1 1 1] Verifica a variável para inverter a direção do movimento e ajusta o tamaho
  (`SceneComponent.SetWorldScale3D` (`self.Sprite`) (`KismetMathLibrary.MakeVector` (* (`KismetMathLibrary.Abs` _returnvalue_x) (select `bool` (`self.bInverterDireção`) :`false` -1.0 :`true` 1.0 :!type "Float (single-precision)")) _returnvalue_y _returnvalue_z)))

(fn `UserConstructionScript`
  (bind _capsulecomponent (`self.CapsuleComponent`))
  (bind _tamanho_do_sprite (`self.Tamanho do Sprite`))
  (bind _tamanho_geral (`self.Tamanho Geral`))
  ;[1 1 1] Configura a vida máxima do inimigo, determina o flipbook e ajusta o tamanho geral
  ; Depois ajusta o tamanho da colisão do inimigo
  ; Por fim, ajusta o tamanho do sprite e a posição
  (set `self.Vida Atual` (`self.Vida Máxima`))
  (`PaperFlipbookComponent.SetFlipbook` (`self.Sprite`) (`self.Andando`))
  (`self.SetActorScale3D` (`KismetMathLibrary.MakeVector` _tamanho_geral _tamanho_geral _tamanho_geral))
  (`CapsuleComponent.SetCapsuleHalfHeight` _capsulecomponent (`self.Altura da colisão`) true)
  (`CapsuleComponent.SetCapsuleRadius` _capsulecomponent (`self.Largura da colisão`) true)
  (`SceneComponent.SetRelativeScale3D` (`self.Sprite`) (`KismetMathLibrary.MakeVector` _tamanho_do_sprite _tamanho_do_sprite _tamanho_do_sprite))
  (`SceneComponent.K2_SetRelativeLocation` (`self.Sprite`) (`KismetMathLibrary.MakeVector` (`self.Posição Horizontal do Sprite`) 0.0 (`self.Posição Vertical do Sprite`)) false false))