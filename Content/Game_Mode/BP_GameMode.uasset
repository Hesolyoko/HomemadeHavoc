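; BP_GameMode is the game mode that keeps the player's score and decides when the game is won.
; On BeginPlay it resets Pontuacao and adds the HUD_Gameplay widget to the viewport.
; GanharPonto adds the given value, refreshes the HUDMoeda coin counter, then runs VerificarVitoria.
; That check calls Vitoria, intended for the gameplay HUD, once the score reaches PontuacaoParaVencer.
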(event `self.ReceiveBeginPlay`
  ;[1 1 1] Zera a pontuação quando inicia o jogo
  (set `self.Pontuacao` 0)
  (bind _returnvalue (`|CreateWidget` "/Game/UI/HUD_Gameplay.HUD_Gameplay_C" (`GameplayStatics.GetPlayerController` 0)))
  (bind _output_get (set `self.HUD Gameplay` _returnvalue))
  (`UserWidget.AddToViewport` _output_get 1))

(fn `Ganhar Ponto`
  (params (Valor :type Integer))
  ;[1 1 1] Acrescenta 1 ao contador de pontos e chama a função de verificar vitória
  (bind _output_get (set `self.Pontuacao` (+ Valor (`self.Pontuacao`))))
  (`/Game/UI/HUD_Contador.Atualiza Contador` (`/Game/UI/HUD_Gameplay.HUD_Moeda` (`self.HUD Gameplay`)) _output_get)
  (`self.Verificar Vitoria`))

(fn `UserConstructionScript`)

(fn `Verificar Vitoria`
  ;[1 1 1] Virifica a quantidade de pontos e se atingiu a pontuação para vencer, chama o evento de Vitoria na HUD Gameplay
  (if (>= (`self.Pontuacao`) (`self.PontuacaoParaVencer`))
    (`self.Vitoria`)))